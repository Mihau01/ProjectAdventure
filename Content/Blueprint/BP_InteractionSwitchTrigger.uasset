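; BP_InteractionSwitchTrigger is an interactable switch that triggers a set of other actors when used.
; Each BPIFBeginInteraction event flips its on/off flag and swaps the Button material, red for on and green for off.
; It then forwards the same interface message to every actor in InteractionActor, without passing the switch state, so each target handles the interaction itself.
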(event `/Game/Interfaces/BPI_InteractionInterface.BPIF_BeginInteraction`
  (bind _output_get (set `self.SwtichOn` (not (`self.SwtichOn`))))
  (`PrimitiveComponent.SetMaterial` (`self.Button`) 0 (select `bool` _output_get :`false` "/Engine/EngineDebugMaterials/VertexColorViewMode_GreenOnly.VertexColorViewMode_GreenOnly" :`true` "/AnimationSharing/AnimSharingRed.AnimSharingRed" :!type "MaterialInterface Object Reference"))
  (for _array_element (`self.InteractionActor`)
    (message `/Game/Interfaces/BPI_InteractionInterface.BPIF_BeginInteraction` _array_element)))

(fn `UserConstructionScript`
  (`parent.UserConstructionScript`))