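; Interactable door, a child Blueprint of an interaction asset, that swings open or closed when interacted with.
; The BPIF begin-interaction event uses MoveComponentTo to rotate the placeholder door component's yaw to DoorRotation over half a second.
; It then flips DoorRotation between -90 and 0 degrees so the next interaction swings the door the other way.
; The construction script only calls the parent's.
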(event `/Game/Interfaces/BPI_InteractionInterface.BPIF_BeginInteraction`
  (`KismetSystemLibrary.MoveComponentTo` (`self.PLCHLDDoorAsset`) (0.0 0.0 0.0) (`KismetMathLibrary.MakeRotator` 0.0 0.0 (`self.DoorRotation`)) false false 0.5)
  (if (== (`self.DoorRotation`) -90.0)
    (set `self.DoorRotation` (+ (`self.DoorRotation`) 90.0))
    (else
      (set `self.DoorRotation` -90.0))))

(fn `UserConstructionScript`
  (`parent.UserConstructionScript`))