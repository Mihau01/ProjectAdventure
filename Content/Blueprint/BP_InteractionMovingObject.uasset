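; BP_InteractionMovingObject is an interactable object whose Cube slides between two positions each time an interaction begins.
; The BPIFBeginInteraction event uses a one-second MoveComponentTo to send the Cube to either ChangeLocationVector or its zero relative location.
; The InteractionHappened flag picks the target and is inverted by the event, making the movement a back-and-forth toggle.
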(event `self.ReceiveBeginPlay`
  (`parent.ReceiveBeginPlay`))

(event `/Game/Interfaces/BPI_InteractionInterface.BPIF_BeginInteraction`
  (`KismetSystemLibrary.MoveComponentTo` (`self.Cube`) (select `bool` (`self.InteractionHappened`) :`false` (`self.ChangeLocationVector`)) (struct) false false 1.0)
  (set `self.InteractionHappened` (not (`self.InteractionHappened`))))

(fn `UserConstructionScript`
  (`parent.UserConstructionScript`))