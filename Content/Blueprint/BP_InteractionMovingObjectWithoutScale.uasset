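; Interactable actor that slides and rotates its Cube between its origin and a configurable offset, without changing scale.
; Each BeginInteraction interface call runs a five-second MoveComponentTo toward the offset location and rotation or back to zero, then flips the InteractionHappened toggle.
; Native scale is cached on BeginPlay, but the scale-change calculation is left unconnected.
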(event `self.ReceiveBeginPlay`
  (`parent.ReceiveBeginPlay`)
  (set `self.NativeScale` (`SceneComponent.K2_GetComponentScale` (`self.Cube`))))

(event `self.BPIF_BeginInteraction`
  (bind _interactionhappened (`self.InteractionHappened`))
  (`KismetSystemLibrary.MoveComponentTo` (`self.Cube`) (select `bool` _interactionhappened :`false` (`self.ChangeLocationVector`)) (select `bool` _interactionhappened :`false` (`self.ChangeRotator`)) false false 5.0)
  (set `self.InteractionHappened` (not (`self.InteractionHappened`))))

(fn `UserConstructionScript`
  (`parent.UserConstructionScript`))