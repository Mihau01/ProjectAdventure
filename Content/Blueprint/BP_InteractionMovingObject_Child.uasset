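; BP_InteractionMovingObject_Child is an interactable object whose Cube toggles between a default and a changed transform.
; Each interface interaction runs a timed MoveComponentTo between zero and the configured relative location and rotation, then sets scale and flips InteractionHappened.
; The changed scale adds ChangeScaleVector to the world scale cached at BeginPlay, while reverting sets unit scale instead of that cached value.
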(event `self.ReceiveBeginPlay`
  (`parent.ReceiveBeginPlay`)
  (set `self.NativeScale` (`SceneComponent.K2_GetComponentScale` (`self.Cube`))))

(event `/Game/Interfaces/BPI_InteractionInterface.BPIF_BeginInteraction`
  (bind _interactionhappened (`self.InteractionHappened`))
  (`KismetSystemLibrary.MoveComponentTo` (`self.Cube`) (select `bool` _interactionhappened :`false` (`self.ChangeLocationVector`)) (select `bool` _interactionhappened :`false` (`self.ChangeRotator`)) false false 5.0)
  (`SceneComponent.SetWorldScale3D` (`self.Cube`) (select `bool` _interactionhappened :`false` (+ (`self.NativeScale`) (`self.ChangeScaleVector`)) :`true` (1.0 1.0 1.0)))
  (set `self.InteractionHappened` (not (`self.InteractionHappened`))))

(fn `UserConstructionScript`
  (`parent.UserConstructionScript`))