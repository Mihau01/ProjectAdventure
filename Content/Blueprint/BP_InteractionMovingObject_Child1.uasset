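; Child variant of an interactable moving object that toggles a Cube component between two transforms on each interaction.
; On the begin-interaction interface event, MoveComponentTo animates the Cube over a fixed duration to either the configured location and rotation or a hardcoded return pose.
; A flag flips each time to alternate the direction.
; BeginPlay caches the Cube's world scale, but the scale-change logic is left unconnected.
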(event `self.ReceiveBeginPlay`
  (`parent.ReceiveBeginPlay`)
  (set `self.NativeScale` (`SceneComponent.K2_GetComponentScale` (`self.Cube`))))

(event `/Game/Blueprint/BP_InteractionAsset.BPIF_BeginInteraction`
  (bind _interactionhappened (`self.InteractionHappened`))
  (`KismetSystemLibrary.MoveComponentTo` (`self.Cube`) (select `bool` _interactionhappened :`false` (`self.ChangeLocationVector`) :`true` (0.0 0.0 0.0)) (select `bool` _interactionhappened :`false` (`self.Change Rotator`) :`true` (struct :`Yaw` 180.0)) false false 2.0)
  (set `self.InteractionHappened` (not (`self.InteractionHappened`))))

(fn `UserConstructionScript`
  (`parent.UserConstructionScript`))